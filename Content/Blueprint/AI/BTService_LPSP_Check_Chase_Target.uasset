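; Behavior tree service that monitors the AI's chase target for being alive and in unobstructed view.
; Each tick it validates the ChaseTarget blackboard actor through its health component, clearing the key if missing or dead.
; For a living target, a slightly raised Camera-channel line trace ignoring both actors sets ChaseTargetInView when nothing blocks it, so other tree logic can avoid actions like firing blind.
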(event EventReceiveTickAI
  (params (OwnerController :type AI%20Controller%20Object%20Reference) (ControlledPawn :type Pawn%20Object%20Reference) (DeltaSeconds :type Float%20%28single-precision%29))
  (Variables|Data|SetControlled ControlledPawn)
  (if (CallFunction|IsTargetValid)
    (bind _result (|CGraphTrace))
    (Class|BTFunctionLibrary|SetBlackboardValueasBool (Variables|Config|GetChase_Target_In_View) (not _result)) ; This tells the rest of the BT that the target\nis indeed in view of the AI. This is helpful so\nthat it does not fire when not seeing the target, \nfor instance.
    (else
      (Class|BTFunctionLibrary|SetBlackboardValueasObject (Variables|Config|GetChase_Target)))))

(fn IsTargetAlive
  (params (Test%20Target :type Actor%20Object%20Reference))
  (bind _returnvalue (Actor|GetComponentbyClass Test%20Target "/Game/Blueprint/ActorComponent/BPAC_LPSP_Health.BPAC_LPSP_Health_C"))
  (Utilities|IsValid Test%20Target
    (:Is%20Valid
      (Utilities|IsValid _returnvalue
        (:Is%20Valid
          (return (Default|IsAlive _returnvalue)))
        (:Is%20Not%20Valid
          (return false))))
    (:Is%20Not%20Valid
      (return false))))

(fn IsTargetValid
  (return (CallFunction|IsTargetAlive (AI|BehaviorTree|GetBlackboardValueasActor (Variables|Config|GetChase_Target)))))