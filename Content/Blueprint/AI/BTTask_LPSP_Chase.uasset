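; Behavior tree task that keeps an AI pawn chasing its blackboard target, aiming except when running.
; An EQS query picks the move destination, taken only if the nav path is not partial.
; Parallel timer loops re-query on lost sight, out-of-range distance, flank angle or periodically while visible.
; A running loop swaps aim for sprint on distant destinations, reverting when a move ends close enough, and the task never calls Finish Execute.
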(event Custom|Event%20On%20Query%20Finished
  (params (QueryInstance :type Env%20Query%20Instance%20Blueprint%20Wrapper%20Object%20Reference) (QueryStatus :type EEnvQueryStatus%20Enum :default "Processing"))
  ;[1 0.3879 0 1 12] On Query Finished
  (bind (_resultlocations _returnvalue) (AI|EQS|GetQueryResultsasLocations QueryInstance))
  (if _returnvalue
    (bind _output_get (Variables|Data|SetMove_Target (Utilities|Array|Get(acopy) _resultlocations)))
    (Utilities|IsPathValid _output_get
      (:True
        (AI|AIMoveTo (Variables|Data|GetControlled) (Variables|Data|GetMove_Target) 0 5.0 false
          (:OnSuccess
            _)
          (:OnFail
            _))
        (CallFunction|TryStopRunning)))))

(event Custom|Event%20Run%20Query
  ;[0.1087 1 0 1 12] Run Query
  (bind _returnvalue (AI|EQS|RunEQSQuery (Variables|Config|GetQuery%20Template) (Variables|Data|GetControlled) "RandomBest5Pct"))
  (EventDispatchers|BindEventtoOnQueryFinishedEvent _returnvalue (EventDispatchers|CreateEvent :!event Custom|Event%20On%20Query%20Finished)))

(event Custom|Event%20Re-Query%20For%20Flank
  ;[0 0.7217 1 1 12] Re-Query For Flank
  (Utilities|IsValid (Variables|Default|GetLook%20Component) :!label _label
    (:Is%20Valid
      (if (and (|CGraphHasTargetPassedFlank) (CallFunction|IsChaseTargetVisible))
        (CallFunction|EventRunQuery))
      (Utilities|FlowControl|Delay 0.2)
      (goto _label))))

(event Custom|Event%20Re-Query%20For%20Interest
  ;[1 0.8201 0.05535 1 12] Re-Query For Interest
  (Utilities|FlowControl|RetriggerableDelay 3.0)
  (if (CallFunction|IsChaseTargetVisible) ; This allows us to skip re-running\nEQS queries for interest if we don't\neven see the Chase_Target.
    (CallFunction|EventRunQuery))
  (CallFunction|EventRe-QueryforInterest))

(event Custom|Event%20Re-Query%20If%20Not%20In%20Range
  ;[1 0 0.7655 1 12] Re-Query If Not In Range
  (if (CallFunction|IsNotinRangeOfChaseTarget)
    (CallFunction|EventRunQuery))
  (Utilities|FlowControl|RetriggerableDelay 0.2)
  (CallFunction|EventRe-QueryifNotinRange))

(event Custom|Event%20Re-Query%20For%20Running
  ;[0 1 0.2805 1 12] Re-Query For Running
  (|CGraphRe-QueryForRunning))

(event Custom|Event%20Re-Query%20For%20Trace
  ;[0.6885 1 0 1 12] Re-Query For Trace
  (if (not (CallFunction|IsChaseTargetVisible))
    (CallFunction|EventRunQuery))
  (Utilities|FlowControl|RetriggerableDelay 0.2)
  (CallFunction|EventRe-QueryforTrace))

(event EventReceiveExecuteAI
  (params (OwnerController :type AI%20Controller%20Object%20Reference) (ControlledPawn :type Pawn%20Object%20Reference))
  ;[0.6674 1 0 1 12] Execute AI
  (Variables|Data|SetOwner%20Controller OwnerController)
  (Variables|Data|SetControlled ControlledPawn)
  (CallFunction|ExecuteAI))

(fn IsNotinRangeOfChaseTarget
  (bind _range_check (Variables|Config|GetRange%20Check))
  (bind (_x _y) (Math|Vector2D|BreakVector2D _range_check))
  (return (not (Math|Float|InRange(Float) (CallFunction|GetDistancetoChaseTarget) _x _y))))

(fn GetDistancetoChaseTarget
  (Utilities|IsValid (Variables|Data|GetControlled)
    (:Is%20Valid
      (Utilities|IsValid (AI|BehaviorTree|GetBlackboardValueasActor (Variables|Config|GetChase_Target))
        (:Is%20Valid
          (return (Math|Vector|Distance(Vector) (Transformation|GetActorLocation (AI|BehaviorTree|GetBlackboardValueasActor (Variables|Config|GetChase_Target))) (Transformation|GetActorLocation (Variables|Data|GetControlled)))))
        (:Is%20Not%20Valid
          (return 0.0))))
    (:Is%20Not%20Valid
      (return 0.0))))

(fn ShouldbeRunningforMoveTarget
  (return (>= (CallFunction|GetDistancetoMoveTarget) (Variables|Config|GetMinimum%20Running%20Distance))))

(fn TryStopRunning
  (Utilities|FlowControl|Sequence
    (:then_0
      (if (and (Variables|Data|GetRunning) (not (CallFunction|ShouldbeRunningforMoveTarget)))
        (Variables|Data|SetRunning false)
        (Class|BPILPSPCHAI|LPSP,AI-TriggerStopRun(Message) (Variables|Data|GetControlled))
        (Class|BPILPSPCHAI|LPSP,AI-TriggerAim(Message) (Variables|Data|GetControlled))
        (CallFunction|EventRe-QueryforRunning)
        (Class|BTFunctionLibrary|SetBlackboardValueasBool (Variables|Config|GetWants_To_Run) false)))
    (:then_1
      (return))))

(fn GetDistancetoMoveTarget
  (Utilities|IsValid (Variables|Data|GetControlled)
    (:Is%20Valid
      (return (Math|Vector|Distance(Vector) (Variables|Data|GetMove_Target) (Transformation|GetActorLocation (Variables|Data|GetControlled)))))
    (:Is%20Not%20Valid
      (return 0.0))))

(fn IsChaseTargetVisible
  (return (Class|BTFunctionLibrary|GetBlackboardValueasBool (Variables|Config|GetChase_Target_In_View))))

(fn ExecuteAI
  (Utilities|FlowControl|Sequence
    (:then_0
      (bind _output_get (Variables|Default|SetLook%20Component (Actor|GetComponentbyClass (Variables|Data|GetControlled) "/Game/Blueprint/ActorComponent/BPSC_LPSP_TP_Looks.BPSC_LPSP_TP_Looks_C")))
      (Utilities|IsValid _output_get
        (:Is%20Valid
          (Class|BPILPSPCHAI|LPSP,AI-TriggerAim(Message) (Variables|Data|GetControlled)) ; When the AI is chasing, it always\naims, that's why we trigger it here.
          (CallFunction|EventRunQuery)
          (CallFunction|EventRe-QueryifNotinRange)
          (CallFunction|EventRe-QueryforInterest)
          (CallFunction|EventRe-QueryforFlank)
          (CallFunction|EventRe-QueryforTrace)
          (CallFunction|EventRe-QueryforRunning))))
    (:then_1
      (return))))