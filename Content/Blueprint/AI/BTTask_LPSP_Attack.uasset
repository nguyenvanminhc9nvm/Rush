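; Behavior Tree task that runs one AI attack, choosing melee, grenade throw or gunfire in that order based on distance to the ChaseTarget blackboard actor.
; Each option checks its flag, range and pawn interface message, with melee requiring CanMelee to be false and grenades adding a coin flip and not-running check.
; Shooting fires for a random duration, or triggers a reload and polls until ammunition returns; aborting stops fire.
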(event Custom|Event%20Try%20Start%20Shooting
  ;[1 0.4333 0.7736 1 12] Try Start Shooting
  (if (Variables|Config|GetCan%20Shoot)
    (if (CallFunction|InFiringRange)
      (bind _returnvalue (Class|BPILPSPCHAI|LPSP,AI-CanStartShooting(Message) (Variables|Data|GetControlled)))
      (if _returnvalue
        (bind _value (Class|BPILPSPPCH|LPSP-IsEquippedAmmunitionEmpty(Message) (Variables|Data|GetControlled)))
        (if _value
          (Class|BPILPSPCHAI|LPSP,AI-TriggerReload(Message) (Variables|Data|GetControlled))
          (Utilities|FlowControl|Delay 0.2 :!label _label)
          (bind _value_2 (Class|BPILPSPPCH|LPSP-IsEquippedAmmunitionEmpty(Message) (Variables|Data|GetControlled)))
          (if _value_2
            (goto _label)
            (else
              (AI|BehaviorTree|FinishExecute true)))
          (else
            (CallFunction|EventFire)))
        (else
          (AI|BehaviorTree|FinishExecute true :!label _label_2)))
      (else
        (goto _label_2)))
    (else
      (goto _label_2))))

(event Custom|Event%20Fire
  ;[0.2735 0.6042 0 1 12] Event Fire
  (Class|BPILPSPCHAI|LPSP,AI-StartShooting(Message) (Variables|Data|GetControlled))
  (Utilities|FlowControl|Delay (CallFunction|LPSP-RandomFloatinVectorRange (Variables|Config|GetFire%20Time%20Range)))
  (Class|BPILPSPCHAI|LPSP,AI-StopShooting(Message) (Variables|Data|GetControlled))
  (AI|BehaviorTree|FinishExecute true))

(event EventReceiveExecuteAI
  (params (OwnerController :type AI%20Controller%20Object%20Reference) (ControlledPawn :type Pawn%20Object%20Reference))
  ;[1 0.9036 0.1062 1 12] Execute AI
  (Variables|Data|SetControlled ControlledPawn)
  (bind _performed (CallFunction|TryPerformMeleeAttack))
  (if (not _performed)
    (bind _performed_2 (CallFunction|TryPerformGrenadeThrow))
    (if (not _performed_2)
      (CallFunction|EventTryStartShooting))))

(event EventReceiveAbortAI
  (params (OwnerController :type AI%20Controller%20Object%20Reference) (ControlledPawn :type Pawn%20Object%20Reference))
  ;[1 0.2292 0 1 12] Abort AI
  (Class|BPILPSPCHAI|LPSP,AI-StopShooting(Message) (Variables|Data|GetControlled)) ; This just makes sure we stop\nthe AI from shooting if the task\nis aborted.
)

(fn InFiringRange
  (bind _firing_range (Variables|Config|GetFiring%20Range))
  (bind (_x _y) (Math|Vector2D|BreakVector2D _firing_range))
  (Utilities|FlowControl|Sequence
    (:then_0
      (bind _returnvalue (Utilities|GetDistancetoChaseTarget)
        (:Is%20Valid
          (return (Math|Float|InRange(Float) _returnvalue _x _y)))))
    (:then_1
      (return false))))

(fn InGrenadeRange
  (bind _grenade_range (Variables|Config|GetGrenade%20Range))
  (bind (_x _y) (Math|Vector2D|BreakVector2D _grenade_range))
  (Utilities|FlowControl|Sequence
    (:then_0
      (bind _returnvalue (Utilities|GetDistancetoChaseTarget)
        (:Is%20Valid
          (return (Math|Float|InRange(Float) _returnvalue _x _y)))))
    (:then_1
      (return false))))

(fn InMeleeRange
  (bind _melee_range (Variables|Config|GetMelee%20Range))
  (bind (_x _y) (Math|Vector2D|BreakVector2D _melee_range))
  (Utilities|FlowControl|Sequence
    (:then_0
      (bind _returnvalue (Utilities|GetDistancetoChaseTarget)
        (:Is%20Valid
          (return (Math|Float|InRange(Float) _returnvalue _x _y)))))
    (:then_1
      (return false))))

(fn TryPerformMeleeAttack
  (Utilities|FlowControl|Sequence
    (:then_0
      (if (not (Variables|Config|GetCan%20Melee))
        (if (CallFunction|InMeleeRange)
          (bind _returnvalue (Class|BPILPSPCHAI|LPSP,AI-CanTriggerMelee(Message) (Variables|Data|GetControlled)))
          (if _returnvalue
            (Class|BPILPSPCHAI|LPSP,AI-TriggerMelee(Message) (Variables|Data|GetControlled))
            (AI|BehaviorTree|FinishExecute true)
            (return true)))))
    (:then_1
      (return false))))

(fn TryPerformGrenadeThrow
  (Utilities|FlowControl|Sequence
    (:then_0
      (if (Variables|Config|GetCan%20Throw%20Grenades)
        (if (CallFunction|InGrenadeRange)
          (bind _returnvalue (Class|BPILPSPCHAI|LPSP,AI-CanTriggerThrowGrenade(Message) (Variables|Data|GetControlled)))
          (if (and _returnvalue (Math|Random|RandomBool))
            (bind _returnvalue_2 (Class|BPILPSPPCH|LPSP-IsRunning(Message) (Variables|Data|GetControlled)))
            (if (not _returnvalue_2)
              (Class|BPILPSPCHAI|LPSP,AI-TriggerThrowGrenade(Message) (Variables|Data|GetControlled))
              (AI|BehaviorTree|FinishExecute true)
              (return true))))))
    (:then_1
      (return false))))