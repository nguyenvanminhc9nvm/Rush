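; Actor component that provides aim assist by reporting a look sensitivity multiplier when its owner aims near a designated assist target.
; While enabled, each tick it picks controller or keyboard data, then sphere-traces from a start and direction supplied by the owner through message calls.
; Assist turns on only if the hit actor reports itself as an assist target.
; The multiplier comes from a curve over the impact point's distance from a point on the aim line, defaulting to one.
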(event EventTick
  (params (DeltaSeconds :type Float%20%28single-precision%29))
  (|CallParentFunction DeltaSeconds)
  (if (Variables|InfimaGames|AimAssister|GetEnabled) ; This little check here is very\nhelpful so we can turn off the component\nmore easily.\n\nWe can even do this at runtime, which would\nbe helpful to have for the options menu,\nfor instance.
    (Utilities|FlowControl|Sequence
      (:then_0
        (bind _value (Class|BPILPSPAimAssisterTarget|IsUsingGamepad(Message) (Components|GetOwner))) ; Depending on the value that we get here, we\ncompletely change the data we use for aim\nassist.\n\nIt is very helpful to have one for keyboard\nand one for controller because the feel should\nbe completely different for the most part.
        (if _value
          (Variables|InfimaGames|Data|SetUsed%20Data (Variables|InfimaGames|AimAssister|GetController%20Data))
          (else
            (Variables|InfimaGames|Data|SetUsed%20Data (Variables|InfimaGames|AimAssister|GetKeyboard%20Data)))))
      (:then_1
        (bind (_location _direction) (Class|BPILPSPAimAssisterTarget|GetTraceParameters(Message) (Variables|InfimaGames|Data|GetOwner))) ; We get the trace parameters from the owner itself,\nso we can determine different trace starts and directions\nper actor if we need to.
        (Variables|InfimaGames|Data|SetTrace%20Location _location)
        (Variables|InfimaGames|Data|SetTrace%20Direction _direction)
        (bind _outhit (Collision|SphereTraceForObjects (Variables|InfimaGames|Data|GetTrace%20Location) (+ (Variables|InfimaGames|Data|GetTrace%20Location) (* (Variables|InfimaGames|Data|GetTrace%20Direction) (Variables|/Game/Blueprint/Aim_Assist/BP_LPSP_Aim_Assist_Data.BP_LPSP_Aim_Assist_Data_C|GetDistance (Variables|InfimaGames|Data|GetUsed%20Data)))) (Variables|/Game/Blueprint/Aim_Assist/BP_LPSP_Aim_Assist_Data.BP_LPSP_Aim_Assist_Data_C|GetRadius (Variables|InfimaGames|Data|GetUsed%20Data)) (Variables|/Game/Blueprint/Aim_Assist/BP_LPSP_Aim_Assist_Data.BP_LPSP_Aim_Assist_Data_C|GetObject%20Types (Variables|InfimaGames|Data|GetUsed%20Data)) false 0 (Variables|InfimaGames|AimAssister|GetDraw%20Debug%20Type))) ; Trace for things that we can use to aim\nassist.
        (Variables|InfimaGames|Data|SetTrace%20Hit _outhit)
        (if (.bBlockingHit (Collision|BreakHitResult (Variables|InfimaGames|Data|GetTrace%20Hit)))
          (bind _value_2 (Class|BPILPSPAimAssistTarget|IsAssistTarget(Message) (.HitActor (Collision|BreakHitResult (Variables|InfimaGames|Data|GetTrace%20Hit))))) ; We only really use this entire component\nfor Actors that are specifically designated\nto be Aim Assist Targets.\n\nThis avoids any kind of weird issues we may\nhave with having a sepparate trace channel or\nobject type.
          (if _value_2
            (Variables|InfimaGames|Data|SetAssist%20On true)
            (else
              (Variables|InfimaGames|Data|SetAssist%20On false)))
          (else
            (Variables|InfimaGames|Data|SetAssist%20On false)))))
    (else
      (Variables|InfimaGames|Data|SetAssist%20On false))))

(event EventBeginPlay
  (|CallParentFunction)
  (Variables|InfimaGames|Data|SetOwner (Components|GetOwner)))

(fn IsAssiston
  (return (Variables|InfimaGames|Data|GetAssist%20On)))

(fn GetSensitivityMultiplier
  (if (Variables|InfimaGames|Data|GetAssist%20On)
    (Utilities|IsValid (Variables|/Game/Blueprint/Aim_Assist/BP_LPSP_Aim_Assist_Data.BP_LPSP_Aim_Assist_Data_C|GetSensitivity%20Curve (Variables|InfimaGames|Data|GetUsed%20Data)) ; The sensitivity curve is what determines how\nmuch the sensitivity multiplier is for a given\ndistance to the target, so not having one does\nnot allow us to calculate anything.
      (:Is%20Valid
        (return (Math|Curves|GetFloatValue (Variables|/Game/Blueprint/Aim_Assist/BP_LPSP_Aim_Assist_Data.BP_LPSP_Aim_Assist_Data_C|GetSensitivity%20Curve (Variables|InfimaGames|Data|GetUsed%20Data)) (Math|Vector|Distance(Vector) (.ImpactPoint (Collision|BreakHitResult (Variables|InfimaGames|Data|GetTrace%20Hit))) (+ (Variables|InfimaGames|Data|GetTrace%20Location) (* (Variables|InfimaGames|Data|GetTrace%20Direction) (+ (.Distance (Collision|BreakHitResult (Variables|InfimaGames|Data|GetTrace%20Hit))) (Variables|/Game/Blueprint/Aim_Assist/BP_LPSP_Aim_Assist_Data.BP_LPSP_Aim_Assist_Data_C|GetRadius (Variables|InfimaGames|Data|GetUsed%20Data)))))))))
      (:Is%20Not%20Valid
        (return 1.0)))
    (else
      (return 1.0))))

(fn SetEnabled
  (params (Value :type Boolean))
  (Variables|InfimaGames|AimAssister|SetEnabled Value)
  (return))