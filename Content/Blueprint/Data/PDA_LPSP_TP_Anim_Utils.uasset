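; Third-person animation utility that decides when movement direction switches between Forward, Backward, Forward Left and Backward Left.
; Each function is one named transition rule that compares MovementAngle to a threshold and returns a boolean.
; The four directions act as quadrants split near zero and ±90 degrees.
; Opposite transitions use thresholds five degrees apart, a hysteresis band that prevents flickering at the boundaries.
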(fn Forward->ForwardLeft
  (params (Movement%20Angle :type Float%20%28double-precision%29))
  (return (< Movement%20Angle -5.0)))

(fn Forward->Backward
  (params (Movement%20Angle :type Float%20%28double-precision%29))
  (return (> Movement%20Angle 95.0)))

(fn Backward->BackwardLeft
  (params (Movement%20Angle :type Float%20%28double-precision%29))
  (return (< Movement%20Angle 0.0)))

(fn Backward->Forward
  (params (Movement%20Angle :type Float%20%28double-precision%29))
  (return (<= Movement%20Angle 9e+01)))

(fn ForwardLeft->BackwardLeft
  (params (Movement%20Angle :type Float%20%28double-precision%29))
  (return (< Movement%20Angle -95.0)))

(fn ForwardLeft->Forward
  (params (Movement%20Angle :type Float%20%28double-precision%29))
  (return (>= Movement%20Angle 0.0)))

(fn BackwardLeft->ForwardLeft
  (params (Movement%20Angle :type Float%20%28double-precision%29))
  (return (>= Movement%20Angle -9e+01)))

(fn BackwardLeft->Backward
  (params (Movement%20Angle :type Float%20%28double-precision%29))
  (return (> Movement%20Angle 5.0)))