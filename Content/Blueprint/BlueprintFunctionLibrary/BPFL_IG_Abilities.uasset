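; Blueprint function library for a lightweight, tag-driven game ability system that works directly on a gameplay tag container.
; An ability can start when the container has all its required tags and none of its blocked tags, using exact matches.
; Starting appends the ability's added tags and strips its removed tags.
; Stopping strips the added tags and optionally restores all removed tags, without tracking which were originally present.
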(fn CanStartGameAbility
  (params (Ability :type S%20Game%20Ability%20Structure) (Container :type Gameplay%20Tag%20Container%20Structure))
  (Utilities|FlowControl|Sequence
    (:then_0
      (if (GameplayTags|HasAllTags Container (Utilities|Struct|BreakSGameAbility Ability) true)
        (if (not (GameplayTags|HasAnyTags Container (Utilities|Struct|BreakSGameAbility Ability) true))
          (return true))))
    (:then_1
      (return false))))

(fn TryStartGameAbility
  (params (Ability :type S%20Game%20Ability%20Structure) (Container :type Gameplay%20Tag%20Container%20Structure%20%28by%20ref%29))
  (Utilities|FlowControl|Sequence
    (:then_0
      (if (InfimaGames|FunctionLibraries|Abilities|CanStartGameAbility Ability Container (LocalVariables|Get__WorldContext))
        (InfimaGames|FunctionLibraries|Abilities|StartGameAbility Ability Container (LocalVariables|Get__WorldContext))
        (return true)))
    (:then_1
      (return false))))

(fn StartGameAbility
  (params (Ability :type S%20Game%20Ability%20Structure) (Container :type Gameplay%20Tag%20Container%20Structure%20%28by%20ref%29))
  (Utilities|FlowControl|Sequence
    (:then_0
      (GameplayTags|AppendGameplayTagContainers Container (Utilities|Struct|BreakSGameAbility Ability))
      (InfimaGames|FunctionLibraries|Abilities|RemoveGameplayTagContainer Container (Utilities|Struct|BreakSGameAbility Ability) (LocalVariables|Get__WorldContext)))
    (:then_1
      (return))))

(fn StopGameAbility
  (params (Ability :type S%20Game%20Ability%20Structure) (Container :type Gameplay%20Tag%20Container%20Structure%20%28by%20ref%29) (Add%20Removed :type Boolean))
  (Utilities|FlowControl|Sequence
    (:then_0
      (InfimaGames|FunctionLibraries|Abilities|RemoveGameplayTagContainer Container (Utilities|Struct|BreakSGameAbility Ability) (LocalVariables|Get__WorldContext))
      (if Add%20Removed
        (GameplayTags|AppendGameplayTagContainers Container (Utilities|Struct|BreakSGameAbility Ability))))
    (:then_1
      (return))))

(fn RemoveGameplayTagContainer
  (params (A :type Gameplay%20Tag%20Container%20Structure%20%28by%20ref%29) (B :type Gameplay%20Tag%20Container%20Structure))
  (Utilities|FlowControl|Sequence
    (:then_0
      (for _array_element (GameplayTags|BreakGameplayTagContainer B)
        (GameplayTags|RemoveGameplayTag A _array_element :!class /Script/GameplayTags.BlueprintGameplayTagLibrary)))
    (:then_1
      (return))))