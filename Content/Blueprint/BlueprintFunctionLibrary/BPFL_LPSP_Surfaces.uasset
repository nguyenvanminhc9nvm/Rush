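; Blueprint function library that spawns surface impact effects from a hit result and a data table row.
; SpawnSurfaceDetails always plays the row's sound if valid, passing the surface type as an int parameter so the sound itself can vary.
; If the row's Details map contains that surface type, it also spawns a fading decal and particle emitters.
; These align to the impact normal, with configured rotation offsets, optional random roll and randomized scale.
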(fn GetRotationfromSettings
  (params (Settings :type S%20Settings%20Structure))
  (bind _rotationoffset (Utilities|Struct|BreakSSettings Settings))
  (bind (_roll _pitch _yaw) (Math|Rotator|BreakRotator _rotationoffset))
  (if (Utilities|Struct|BreakSSettings Settings)
    (return (Math|Rotator|MakeRotator (+ _roll (Math|Random|RandomFloatinRange 0.0 3.6e+02)) _pitch _yaw))
    (else
      (return (Utilities|Struct|BreakSSettings Settings)))))

(fn SpawnSurfaceDetails
  (params (Result :type Hit%20Result%20Structure) (Row%20Handle :type Data%20Table%20Row%20Handle%20Structure))
  (bind (_datatable _rowname) (Utilities|Struct|BreakDataTableRowHandle Row%20Handle))
  (bind _returnvalue (Utilities|GetDataTableRow _datatable _rowname)
    (:then
      (LocalVariables|SetSurfaces _returnvalue)
      (|CGraphGetHitResultValues)
      (|CGraphSpawnSound)
      (LocalVariables|SetDetails (.Value (Utilities|Map|Find (Utilities|Struct|BreakSSurfaces (LocalVariables|GetSurfaces)) (Collision|GetSurfaceType Result))))
      (if (.ReturnValue (Utilities|Map|Find (Utilities|Struct|BreakSSurfaces (LocalVariables|GetSurfaces)) (Collision|GetSurfaceType Result)))
        (|CGraphSpawnDecal)
        (|CGraphSpawnParticles)))))