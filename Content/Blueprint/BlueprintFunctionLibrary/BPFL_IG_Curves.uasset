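; Blueprint function library of curve helpers that configure Timeline components from float or vector curve data.
; Each function takes a curve struct holding a curve and a track name, then assigns that curve to the named track on the given timeline.
; Both set the timeline length mode to last keyframe, so its duration follows the curve's keys.
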(fn SetUpCurveFloat
  (params (Timeline%20Component :type Timeline%20Component%20Object%20Reference%20%28by%20ref%29) (Curve :type S%20Curve%20Float%20Structure))
  (bind (_floattrackname _floatcurve) (Utilities|Struct|BreakSCurveFloat Curve))
  (Utilities|FlowControl|Sequence
    (:then_0
      (Class|TimelineComponent|SetFloatCurve Timeline%20Component _floatcurve _floattrackname)
      (Class|TimelineComponent|SetTimelineLengthMode Timeline%20Component "TL_LastKeyFrame"))
    (:then_1
      (return))))

(fn SetUpCurveVector
  (params (Timeline%20Component :type Timeline%20Component%20Object%20Reference%20%28by%20ref%29) (Curve :type S%20Curve%20Vector%20Structure))
  (bind (_vectortrackname _vectorcurve) (Utilities|Struct|BreakSCurveVector Curve))
  (Utilities|FlowControl|Sequence
    (:then_0
      (Class|TimelineComponent|SetVectorCurve Timeline%20Component _vectorcurve _vectortrackname)
      (Class|TimelineComponent|SetTimelineLengthMode Timeline%20Component "TL_LastKeyFrame"))
    (:then_1
      (return))))