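; Function library of helpers that pick third-person (TP) lag values from an LPSP animation settings input.
; Standing and aiming getters each return the TP lag when an override flag is set, otherwise the default lag.
; Both getters test the standing-lag override flag, so it also controls aiming lag.
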(fn LPSP-GetStandingLagTP
  (params (Settings :type S%20Settings%20Animation%20Structure))
  (if (.OverrideTPStandingLag (Utilities|Struct|BreakS_Settings_Animation Settings))
    (return (.TPStandingLag (Utilities|Struct|BreakS_Settings_Animation Settings)))
    (else
      (return (.StandingLag (Utilities|Struct|BreakS_Settings_Animation Settings))))))

(fn LPSP-GetAimingLagTP
  (params (Settings :type S%20Settings%20Animation%20Structure))
  (if (.OverrideTPStandingLag (Utilities|Struct|BreakS_Settings_Animation Settings))
    (return (.TPAimingLag (Utilities|Struct|BreakS_Settings_Animation Settings)))
    (else
      (return (.AimingLag (Utilities|Struct|BreakS_Settings_Animation Settings))))))