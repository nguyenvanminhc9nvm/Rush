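; Blueprint function library of LPSP math helpers for rotators, transforms, vectors, ranged random values and spring interpolation.
; Rotator and transform math works component-wise instead of composing rotations, with transform addition resetting scale to one and negation optionally preserving it.
; Random helpers read a vector's X and Y as min and max.
; Float and vector spring wrappers take stiffness, damping and mass from one data struct.
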(fn LPSP-AddRotators
  (params (A :type Rotator) (B :type Rotator))
  (bind (_roll _pitch _yaw) (Math|Rotator|BreakRotator A))
  (bind (_roll_2 _pitch_2 _yaw_2) (Math|Rotator|BreakRotator B))
  (return (Math|Rotator|MakeRotator (+ _roll _roll_2) (+ _pitch _pitch_2) (+ _yaw _yaw_2))))

(fn LPSP-NegateRotator
  (params (A :type Rotator))
  (return (* A -1.0)))

(fn LPSP-AddTransforms
  (params (A :type Transform) (B :type Transform))
  (bind (_location _rotation) (Math|Transform|BreakTransform A))
  (bind (_location_2 _rotation_2) (Math|Transform|BreakTransform B))
  (return (Math|Transform|MakeTransform (+ _location _location_2) (InfimaGames|FunctionLibraries|Math|Pure|LPSP-AddRotators _rotation _rotation_2 (LocalVariables|Get__WorldContext)))))

(fn LPSP-VectortoRotator
  (params (In :type Vector))
  (bind (_x _y _z) (Math|Vector|BreakVector In))
  (return (Math|Rotator|MakeRotator _x _y _z)))

(fn LPSP-RotatortoVector
  (params (Value :type Rotator))
  (bind (_roll _pitch _yaw) (Math|Rotator|BreakRotator Value))
  (return (Math|Vector|MakeVector _roll _pitch _yaw)))

(fn LPSP-RandomFloatinVectorRange
  (params (Range :type Vector%202D%20Structure))
  (bind (_x _y) (Math|Vector2D|BreakVector2D Range))
  (return (Math|Random|RandomFloatinRange _x _y)))

(fn LPSP-RandomIntegerinVectorRange
  (params (Range :type Vector%202D%20Structure))
  (bind (_x _y) (Math|Vector2D|BreakVector2D Range))
  (return (Math|Random|RandomIntegerinRange (Math|Float|Truncate _x) (Math|Float|Truncate _y))))

(fn LPSP-NegateTransform
  (params (In :type Transform) (Ignore%20Scale :type Boolean))
  (bind (_location _rotation _scale) (Math|Transform|BreakTransform In))
  (return (Math|Transform|MakeTransform (Math|Vector|NegateVector _location) (InfimaGames|FunctionLibraries|Math|Pure|LPSP-NegateRotator _rotation (LocalVariables|Get__WorldContext)) (select Ignore%20Scale _scale (Math|Vector|NegateVector _scale)))))

(fn LPSP-SubtractRotators
  (params (A :type Rotator) (B :type Rotator))
  (bind (_roll _pitch _yaw) (Math|Rotator|BreakRotator A))
  (bind ___worldcontext (LocalVariables|Get__WorldContext))
  (bind _returnvalue (InfimaGames|FunctionLibraries|Math|Pure|LPSP-NegateRotator B ___worldcontext))
  (bind (_roll_2 _pitch_2 _yaw_2) (Math|Rotator|BreakRotator _returnvalue))
  (return (Math|Rotator|MakeRotator (+ _roll _roll_2) (+ _pitch _pitch_2) (+ _yaw _yaw_2))))

(fn LPSP-CustomFloatSpringInterp
  (params (Current :type Float%20%28double-precision%29) (Target :type Float%20%28double-precision%29) (Delta%20Time :type Float%20%28double-precision%29) (Data :type S%20Spring%20Interp%20Vector%20Structure) (Spring%20State :type Float%20Spring%20State%20Structure%20%28by%20ref%29))
  (LocalVariables|SetLocal%20Data Data)
  (bind _returnvalue (Class|KismetMathLibrary|FloatSpringInterp Current Target Spring%20State (.Stiffness (Utilities|Struct|BreakSSpringInterpVector (LocalVariables|GetLocal%20Data))) (.CriticalDampingFactor (Utilities|Struct|BreakSSpringInterpVector (LocalVariables|GetLocal%20Data))) Delta%20Time (.Mass (Utilities|Struct|BreakSSpringInterpVector (LocalVariables|GetLocal%20Data))) 1.0))
  (return _returnvalue))

(fn LPSP-CustomVectorSpringInterp
  (params (Current :type Vector) (Target :type Vector) (Delta%20Time :type Float%20%28double-precision%29) (Data :type S%20Spring%20Interp%20Vector%20Structure) (Spring%20State :type Vector%20Spring%20State%20Structure%20%28by%20ref%29))
  (LocalVariables|SetLocal%20Data Data)
  (bind _returnvalue (Class|KismetMathLibrary|VectorSpringInterp Current Target Spring%20State (.Stiffness (Utilities|Struct|BreakSSpringInterpVector (LocalVariables|GetLocal%20Data))) (.CriticalDampingFactor (Utilities|Struct|BreakSSpringInterpVector (LocalVariables|GetLocal%20Data))) Delta%20Time (.Mass (Utilities|Struct|BreakSSpringInterpVector (LocalVariables|GetLocal%20Data))) 0.0))
  (return _returnvalue))

(fn LPSP-GetYawRotator
  (params (A :type Rotator))
  (return (Math|Rotator|MakeRotator 0.0 0.0 (.Yaw (Math|Rotator|BreakRotator A)))))

(fn LPSP-toYawRotator
  (params (Yaw :type Float%20%28double-precision%29))
  (return (Math|Rotator|MakeRotator 0.0 0.0 Yaw)))