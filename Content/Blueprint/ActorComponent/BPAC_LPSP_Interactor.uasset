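; Actor component that detects what its owner can interact with, storing the hit result and interaction type for other code to read.
; Each tick it gets location and forward from the owner through interface messages and, if enabled and permitted, sphere-traces ahead.
; On a miss, a Character owner gets a fallback sphere trace at the capsule's base.
; Hit actors report their type through interface messages, otherwise the type resets.
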(event EventTick
  (params (DeltaSeconds :type Float%20%28single-precision%29))
  (|CallParentFunction DeltaSeconds)
  (Utilities|IsValid (Variables|InfimaGames|LowPolyShooterPack|Data|GetOwner)
    (:Is%20Valid
      (Utilities|FlowControl|Sequence
        (:then_0
          (bind (_location _forward) (Class|BPILPSPInteractorTarget|LPSP-GetInteractVectors(Message) (Variables|InfimaGames|LowPolyShooterPack|Data|GetOwner)))
          (Variables|InfimaGames|LowPolyShooterPack|Data|SetLocation _location)
          (Variables|InfimaGames|LowPolyShooterPack|Data|SetForward _forward)
          (|CGraphTrace))
        (:then_1
          (bind _ascharacter (Utilities|Casting|CastToCharacter (Variables|InfimaGames|LowPolyShooterPack|Data|GetOwner)))
          (Variables|InfimaGames|LowPolyShooterPack|Data|SetCharacter _ascharacter))))))

(event EventBeginPlay
  (|CallParentFunction)
  (Variables|InfimaGames|LowPolyShooterPack|Data|SetOwner (Components|GetOwner)))

(fn ResetType
  (Utilities|FlowControl|Sequence
    (:then_0
      (Variables|InfimaGames|LowPolyShooterPack|Data|SetType "NewEnumerator2"))
    (:then_1
      (return))))

(fn TryAssignType
  (Utilities|FlowControl|Sequence
    (:then_0
      (bind _returnvalue (Class|BPILPSPInteractable|CanInteract(Message) (.HitActor (Collision|BreakHitResult (Variables|InfimaGames|LowPolyShooterPack|Data|GetHit%20Result)))))
      (if _returnvalue
        (bind _type (Class|BPILPSPInteractable|GetInteractionType(Message) (.HitActor (Collision|BreakHitResult (Variables|InfimaGames|LowPolyShooterPack|Data|GetHit%20Result)))))
        (Variables|InfimaGames|LowPolyShooterPack|Data|SetType _type)
        (else
          (InfimaGames|LowPolyShooterPack|Interactor|ResetType))))
    (:then_1
      (return))))

(fn SetDistance
  (params (Value :type Float%20%28double-precision%29))
  (Variables|InfimaGames|LowPolyShooterPack|Interactor|SetDistance Value)
  (return))

(fn LPSP-GetHitResult
  (return (Variables|InfimaGames|LowPolyShooterPack|Data|GetHit%20Result)))

(fn LPSP-GetType
  (return (Variables|InfimaGames|LowPolyShooterPack|Data|GetType)))