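; Actor component that computes and replicates third-person body yaw and spine look rotations for LPSP players and AI.
; On the locally controlled owner, a Delay loop at the tick interval replaces Event Tick.
; Players derive values from camera, aim trace, movement and a turn-in-place yaw threshold; AI uses velocity and chase-target facing.
; Smoothed results apply locally, then pass through server events to multicasts that skip the local owner.
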(event Custom|Event%20Update
  (InfimaGames|ThirdPersonLooksComponent|GetOwnerValues)
  (InfimaGames|ThirdPersonLooksComponent|UpdateRootYawMoving)
  (bind _returnvalue (Class|BPILPSPPCH|LPSP-IsAI(Message) (Components|GetOwner))) ; We need to check whether this is an AI,\nas we run this component on both players\nand AI.
  (if _returnvalue
    (InfimaGames|ThirdPersonLooksComponent|AIUpdate)
    (else
      (InfimaGames|ThirdPersonLooksComponent|LocalUpdate))))

(event Custom|Event%20Owner%20Posessed
  (bind _local (Class|BPILPSPPCH|LPSP-IsLocal(Message) (Components|GetOwner)))
  (if _local
    (CallFunction|EventLocalInit)
    ;[1 0.9141 0 1 12] These nodes are what we use instead of using the Event Tick to update stuff. This is helpful because it makes us able to better control update rate.
    (Utilities|FlowControl|Delay (Class|ActorComponent|GetComponentTickInterval) :!label _label)
    (CallFunction|EventUpdate)
    (goto _label)))

(event Custom|Event%20Smoothly%20Set%20Root%20Yaw%20Moving%20Smooth
  (params (Target :type Rotator))
  (CallFunction|EventAllSetRootYawMovingSmooth (Math|Rotator|MakeRotator 0.0 0.0 (.Yaw (Math|Rotator|BreakRotator (Math|Interpolation|RInterpTo (Variables|InfimaGames|Data|GetRoot%20Yaw%20Moving%20Smooth) Target (Utilities|Time|GetWorldDeltaSeconds) 1e+01))))))

(event Custom|Event%20Local%20Init
  ;[1 0.8672 0 1 12] Init
  (|CGraphFixSpawnRotation))

(event Custom|Event%20Multicast%20Set%20Fully%20Holstered%20Pitch
  (params (Value :type Float%20%28double-precision%29))
  ;[1 0.635 0 1 12] Set Fully Holstered Pitch
  (bind _local (Class|BPILPSPPCH|LPSP-IsLocal(Message) (Components|GetOwner)))
  (if (not _local)
    (Variables|InfimaGames|Data|SetFully%20Holstered%20Pitch Value)))

(event Custom|Event%20All%20Set%20Root%20Yaw%20Moving%20Smooth
  (params (Value :type Rotator))
  ;[0 1 0.7656 1 12] Set Root Yaw Moving Smooth. Updates the value!
  (Variables|InfimaGames|Data|SetRoot%20Yaw%20Moving%20Smooth Value)
  (CallFunction|EventServerSetRootYawMovingSmooth (Variables|InfimaGames|Data|GetRoot%20Yaw%20Moving%20Smooth)))

(event Custom|Event%20Multicast%20Set%20Look%20Moving
  (params (Value :type Rotator))
  ;[0.9219 1 0 1 12] Set Look Moving. Updates the value!
  (bind _local (Class|BPILPSPPCH|LPSP-IsLocal(Message) (Components|GetOwner)))
  (if (not _local)
    (Variables|InfimaGames|Data|SetLook%20Moving Value)))

(event Custom|Event%20All%20Set%20Look%20Moving
  (params (Value :type Rotator))
  ;[0.9219 1 0 1 12] Set Look Moving. Updates the value!
  (Variables|InfimaGames|Data|SetLook%20Moving Value)
  (CallFunction|EventServerSetLookMoving Value))

(event Custom|Event%20Server%20Set%20Root%20Yaw%20Moving%20Smooth
  (params (Value :type Rotator))
  ;[0 1 0.7656 1 12] Set Root Yaw Moving Smooth. Updates the value!
  (CallFunction|EventMulticastSetRootYawMovingSmooth Value))

(event Custom|Event%20Server%20Set%20Look%20Moving
  (params (Value :type Rotator))
  ;[0.9219 1 0 1 12] Set Look Moving. Updates the value!
  (CallFunction|EventMulticastSetLookMoving Value))

(event Custom|Event%20Multicast%20Set%20Root%20Yaw%20Moving%20Smooth
  (params (Value :type Rotator))
  ;[0 1 0.7656 1 12] Set Root Yaw Moving Smooth. Updates the value!
  (bind _local (Class|BPILPSPPCH|LPSP-IsLocal(Message) (Components|GetOwner)))
  (if (not _local)
    (Variables|InfimaGames|Data|SetRoot%20Yaw%20Moving%20Smooth Value)))

(event Custom|Event%20Multicast%20Set%20Normalized%20Yaw%20Time
  (params (Value :type Float%20%28double-precision%29))
  ;[0.7988 1 0 1 12] Set Normalized Yaw Time
  (bind _local (Class|BPILPSPPCH|LPSP-IsLocal(Message) (Components|GetOwner)))
  (if (not _local)
    (Variables|InfimaGames|Data|SetNormalized%20Yaw%20Time Value)))

(event Custom|Event%20%28Server%29%20Set%20Fully%20Holstered%20Pitch
  (params (Value :type Float%20%28double-precision%29))
  ;[1 0.635 0 1 12] Set Fully Holstered Pitch
  (CallFunction|EventMulticastSetFullyHolsteredPitch Value))

(event Custom|Event%20%28All%29%20Set%20Normalized%20Yaw%20Time
  (params (Value :type Float%20%28double-precision%29))
  ;[0.7988 1 0 1 12] Set Normalized Yaw Time
  (Variables|InfimaGames|Data|SetNormalized%20Yaw%20Time Value)
  (CallFunction|Event(Server)SetNormalizedYawTime Value))

(event Custom|Event%20%28All%29%20Set%20Fully%20Holstered%20Pitch
  (params (Value :type Float%20%28double-precision%29))
  ;[1 0.635 0 1 12] Set Fully Holstered Pitch
  (Variables|InfimaGames|Data|SetFully%20Holstered%20Pitch Value)
  (CallFunction|Event(Server)SetFullyHolsteredPitch Value))

(event Custom|Event%20%28Server%29%20Set%20Normalized%20Yaw%20Time
  (params (Value :type Float%20%28double-precision%29))
  ;[0.7988 1 0 1 12] Set Normalized Yaw Time
  (CallFunction|EventMulticastSetNormalizedYawTime Value))

(fn GetSpineAddedRotation
  (Utilities|FlowControl|Sequence
    (:then_0
      (Utilities|IsValid (Variables|Default|GetOwning%20Camera)
        (:Is%20Valid
          (bind _equipped_item (Class|BPILPSPPCH|LPSP-GetEquippedItem(Message) (Components|GetOwner)))
          (Utilities|IsValid _equipped_item
            (:Is%20Valid
              (LocalVariables|SetItem%20Location (Transformation|GetActorLocation _equipped_item))
              (return (Math|Rotator|Delta(Rotator) (Math|Rotator|FindLookatRotation (LocalVariables|GetItem%20Location) (Variables|InfimaGames|Data|GetImpact)) (Transformation|GetWorldRotation (Variables|Default|GetOwning%20Camera)))))))))
    (:then_1
      (return "0.000000,0.000000,0.000000"))))

(fn GetLookImpact
  (bind _owning_camera (Variables|Default|GetOwning%20Camera))
  (bind _returnvalue (Transformation|GetWorldLocation _owning_camera))
  (bind _returnvalue_2 (Math|Vector|GetForwardVector _owning_camera))
  (Utilities|FlowControl|Sequence
    (:then_0
      (Utilities|IsValid (Variables|Default|GetOwning%20Camera)
        (:Is%20Valid
          (bind _outhit (Collision|LineTraceByChannel (+ _returnvalue (* _returnvalue_2 1e+01)) (+ _returnvalue (* _returnvalue_2 (Variables|InfimaGames|Config|GetMaximum%20Trace%20Range))) "TraceTypeQuery1" false (Utilities|Array|MakeArray (Components|GetOwner)) "None"))
          (return (.bBlockingHit (Collision|BreakHitResult _outhit)) (.ImpactPoint (Collision|BreakHitResult _outhit))))))
    (:then_1
      (return false "0, 0, 0"))))

(fn GetLook
  (params (Root%20Yaw :type Rotator))
  (bind (_roll _pitch _yaw) (Math|Rotator|BreakRotator Root%20Yaw))
  (return (Math|Rotator|MakeRotator (Math|Float|Clamp(Float) (.Pitch (Math|Rotator|BreakRotator (* (InfimaGames|ThirdPersonLooksComponent|GetCameraLookSpineAdded) -1))) -89.900002 89.900002) 0.0 (- (.Yaw (Math|Rotator|BreakRotator (Math|Rotator|Delta(Rotator) (InfimaGames|ThirdPersonLooksComponent|GetCameraLookSpineAdded) (Math|Rotator|MakeRotator _roll _pitch _yaw)))) 9e+01))))

(fn GetCameraLookSpineAdded
  (return (CallFunction|LPSP-AddRotators (Variables|InfimaGames|Data|GetCamera%20Look%20Smooth) (Math|Rotator|SelectRotator "0, 0, 0" (Variables|InfimaGames|Data|GetSpine%20Added%20Rotation) (Variables|InfimaGames|Data|GetFully%20Holstered)))))

(fn SetImpact
  (bind (_hit _impact) (InfimaGames|ThirdPersonLooksComponent|GetLookImpact))
  (Utilities|FlowControl|Sequence
    (:then_0
      (Utilities|IsValid (Variables|Default|GetOwning%20Camera)
        (:Is%20Valid
          (Variables|InfimaGames|Data|SetImpact (Math|Vector|SelectVector _impact (+ (Transformation|GetWorldLocation) (* (Math|Vector|GetForwardVector (Variables|Default|GetOwning%20Camera)) 1e+04)) _hit))
          (return))))
    (:then_1
      (return))))

(fn GetOwnerValues
  (Utilities|FlowControl|Sequence
    (:then_0
      (Utilities|FlowControl|Sequence
        (:then_0
          ;[0.9453 1 0 1 12] Update the owning camera.
          (Utilities|IsValid (Variables|Default|GetOwning%20Camera)
            (:Is%20Not%20Valid
              (Variables|Default|SetOwning%20Camera (Actor|GetComponentbyClass (Components|GetOwner) "/Script/Engine.CameraComponent")))))
        (:then_1
          (Utilities|FlowControl|Sequence
            (:then_0
              (bind _returnvalue (Class|BPILPSPPCH|LPSP-GetInputMovement(Message) (Components|GetOwner)))
              (Variables|InfimaGames|Data|SetMovement _returnvalue)
              (InfimaGames|ThirdPersonLooksComponent|SetImpact)
              (Variables|InfimaGames|Data|SetSpine%20Added%20Rotation (Math|Interpolation|RInterpTo (Variables|InfimaGames|Data|GetSpine%20Added%20Rotation) (InfimaGames|ThirdPersonLooksComponent|GetSpineAddedRotation) (Utilities|Time|GetWorldDeltaSeconds) (Variables|InfimaGames|Config|GetProcedural%20Component%20Interpolation)))
              (bind _owning_camera (Variables|Default|GetOwning%20Camera)
                (:then
                  (Variables|InfimaGames|Data|SetCamera%20Look%20Smooth (Math|Interpolation|RInterpTo (Variables|InfimaGames|Data|GetCamera%20Look%20Smooth) (Transformation|GetWorldRotation _owning_camera) (Utilities|Time|GetWorldDeltaSeconds) (Variables|InfimaGames|Config|GetLook%20Interpolation))))
                (:else
                  _))
              (Variables|InfimaGames|Data|SetOwner%20Forward (Math|Transform|TransformRotation (Transformation|GetActorTransform (Components|GetOwner)) "0,-90.000000, 0"))
              (Variables|InfimaGames|Data|SetIs%20Moving (!= (Math|Vector2D|Vector2DLength (Variables|InfimaGames|Data|GetMovement)) 0.0))
              (bind _returnvalue_2 (Class|BPILPSPPCH|LPSP-IsThirdPerson(Message) (Components|GetOwner)))
              (Variables|InfimaGames|Data|SetThird%20Person _returnvalue_2)
              (bind _returnvalue_3 (Class|BPILPSPPCH|LPSP-IsAiming(Message) (Components|GetOwner)))
              (Variables|InfimaGames|Data|SetAiming (or _returnvalue_3 (Variables|InfimaGames|Data|GetHolding%20Fire)))
              (bind _returnvalue_4 (Class|BPILPSPPCH|LPSP-IsRunning(Message) (Components|GetOwner)))
              (Variables|InfimaGames|Data|SetRunning _returnvalue_4)
              (bind _is_holding_fire (Class|BPILPSPPCH|LPSP-IsHoldingFire(Message) (Components|GetOwner)))
              (Variables|InfimaGames|Data|SetHolding%20Fire _is_holding_fire))
            (:then_1
              (bind _value (Class|BPILPSPPCH|LPSP-IsFullyHolstered(Message) (Components|GetOwner)))
              (Variables|InfimaGames|Data|SetFully%20Holstered _value)
              (bind _returnvalue_5 (Class|BPILPSPPCH|LPSP-IsUnarmed(Message) (Components|GetOwner)))
              (Variables|InfimaGames|Data|SetUnarmed _returnvalue_5))))))
    (:then_1
      (return))))

(fn UpdateRootYawMoving
  (bind _fully_holstered (Variables|InfimaGames|Data|GetFully%20Holstered))
  (bind _movement (Variables|InfimaGames|Data|GetMovement))
  (bind (_x _y) (Math|Vector2D|BreakVector2D _movement))
  (bind _returnvalue (Math|Float|SelectFloat 65.0 1.1e+02 _fully_holstered))
  (Variables|InfimaGames|Data|SetRoot%20Yaw%20Moving (Math|Rotator|SelectRotator (Math|Rotator|MakeRotator 0.0 0.0 (.Yaw (Math|Rotator|BreakRotator (Math|Transform|TransformRotation (Transformation|GetWorldTransform) (select (Variables|InfimaGames|Data|GetThird%20Person) (Math|Rotator|SelectRotator "0,-90.000000, 0" (Math|Conversions|RotationFromXVector (Math|Vector|MakeVector _x (* _y -1.0) 0.0)) (or (Variables|InfimaGames|Data|GetAiming) (and (Variables|InfimaGames|Data|GetUnarmed) (not (Variables|InfimaGames|Data|GetRunning))))) "0,-90.000000, 0"))))) (CallFunction|LPSP-AddRotators (Variables|InfimaGames|Data|GetRoot%20Yaw%20Moving) (select (Variables|InfimaGames|Data|GetThird%20Person) (CallFunction|LPSP-toYawRotator (select (> (Math|Float|Absolute(Float) (Math|Float|ClampAngle (.Yaw (Math|Rotator|BreakRotator (CallFunction|LPSP-SubtractRotators (Math|Rotator|Delta(Rotator) (CallFunction|LPSP-GetYawRotator (InfimaGames|ThirdPersonLooksComponent|GetCameraLookSpineAdded)) (Variables|InfimaGames|Data|GetRoot%20Yaw%20Moving)) "0,90.000000, 0"))) -1.3e+02 1.3e+02)) _returnvalue) (* (- (Math|Float|Absolute(Float) (Math|Float|ClampAngle (.Yaw (Math|Rotator|BreakRotator (CallFunction|LPSP-SubtractRotators (Math|Rotator|Delta(Rotator) (CallFunction|LPSP-GetYawRotator (InfimaGames|ThirdPersonLooksComponent|GetCameraLookSpineAdded)) (Variables|InfimaGames|Data|GetRoot%20Yaw%20Moving)) "0,90.000000, 0"))) -1.3e+02 1.3e+02)) _returnvalue) (Math|Float|Sign(Float) (Math|Float|ClampAngle (.Yaw (Math|Rotator|BreakRotator (CallFunction|LPSP-SubtractRotators (Math|Rotator|Delta(Rotator) (CallFunction|LPSP-GetYawRotator (InfimaGames|ThirdPersonLooksComponent|GetCameraLookSpineAdded)) (Variables|InfimaGames|Data|GetRoot%20Yaw%20Moving)) "0,90.000000, 0"))) -1.3e+02 1.3e+02))) 0.0)) (CallFunction|LPSP-toYawRotator (select (> (Math|Float|Absolute(Float) (Math|Float|ClampAngle (.Yaw (Math|Rotator|BreakRotator (CallFunction|LPSP-SubtractRotators (Math|Rotator|Delta(Rotator) (CallFunction|LPSP-GetYawRotator (InfimaGames|ThirdPersonLooksComponent|GetCameraLookSpineAdded)) (Variables|InfimaGames|Data|GetRoot%20Yaw%20Moving)) "0,90.000000, 0"))) -1.3e+02 1.3e+02)) _returnvalue) (* (- (Math|Float|Absolute(Float) (Math|Float|ClampAngle (.Yaw (Math|Rotator|BreakRotator (CallFunction|LPSP-SubtractRotators (Math|Rotator|Delta(Rotator) (CallFunction|LPSP-GetYawRotator (InfimaGames|ThirdPersonLooksComponent|GetCameraLookSpineAdded)) (Variables|InfimaGames|Data|GetRoot%20Yaw%20Moving)) "0,90.000000, 0"))) -1.3e+02 1.3e+02)) _returnvalue) (Math|Float|Sign(Float) (Math|Float|ClampAngle (.Yaw (Math|Rotator|BreakRotator (CallFunction|LPSP-SubtractRotators (Math|Rotator|Delta(Rotator) (CallFunction|LPSP-GetYawRotator (InfimaGames|ThirdPersonLooksComponent|GetCameraLookSpineAdded)) (Variables|InfimaGames|Data|GetRoot%20Yaw%20Moving)) "0,90.000000, 0"))) -1.3e+02 1.3e+02))) 0.0)))) (Variables|InfimaGames|Data|GetIs%20Moving)))
  (return))

(fn LocalUpdate
  (Utilities|FlowControl|Sequence
    (:then_0
      (CallFunction|EventAllSetRootYawMovingSmooth (Math|Interpolation|RInterpTo (Variables|InfimaGames|Data|GetRoot%20Yaw%20Moving%20Smooth) (Variables|InfimaGames|Data|GetRoot%20Yaw%20Moving) (Utilities|Time|GetWorldDeltaSeconds) (select (or (Variables|InfimaGames|Data|GetAiming) (Variables|InfimaGames|Data|GetUnarmed)) 15.0 (Math|Float|SelectFloat 2e+01 1e+01 (Variables|InfimaGames|Data|GetRunning)))))
      ;[1 0 0.7734 1 12] This updates the moving look every frame!
      (CallFunction|EventAllSetLookMoving (InfimaGames|ThirdPersonLooksComponent|GetLook (Variables|InfimaGames|Data|GetRoot%20Yaw%20Moving%20Smooth)))
      (CallFunction|Event(All)SetNormalizedYawTime (Math|Float|MapRangeClamped (Math|Float|Absolute(Float) (+ (.Yaw (Math|Rotator|BreakRotator (Variables|InfimaGames|Data|GetLook%20Moving))) 9e+01)) 0.0 1.8e+02 0.0 1.0))
      (CallFunction|Event(All)SetFullyHolsteredPitch (* (.Roll (Math|Rotator|BreakRotator (Variables|InfimaGames|Data|GetLook%20Moving))) -1.0)))
    (:then_1
      (return))))

(fn AIUpdate
  (Utilities|FlowControl|Sequence
    (:then_0
      (Utilities|FlowControl|Sequence
        (:then_0
          (bind _returnvalue (Class|BPILPSPPCH|LPSP-IsMoving(Message) (Components|GetOwner)))
          (if _returnvalue ; We check if the character is moving\nbefore we update its rotation\nfor the velocity. This way we avoid\nrotation changing while standing\nstill.
            (InfimaGames|ThirdPersonLooksComponent|AIUpdateRotationforVelocity)))
        (:then_1
          (bind _returnvalue_2 (Class|BPILPSPCHAI|LPSP,AI-HasValidChaseTarget(Message) (Components|GetOwner)))
          (if _returnvalue_2 ; This check is necessary to\navoid trying to look at a\ntarget that doesn't exist.
            (InfimaGames|ThirdPersonLooksComponent|AIUpdateLook)))))
    (:then_1
      (return))))

(fn AIUpdateRotationforVelocity
  (Utilities|FlowControl|Sequence
    (:then_0
      (bind _returnvalue (Class|BPILPSPPCH|LPSP-GetVelocityRotation(Message) (Components|GetOwner)))
      (LocalVariables|SetAdjusted%20Velocity%20Rotation (CallFunction|LPSP-SubtractRotators _returnvalue "0,90.000000, 0")) ; This value is the rotation that the character\nneeds to have in order to face exactly where\nit is moving.
      (bind _returnvalue_2 (Class|BPILPSPCHAI|LPSP,AI-HasValidChaseTarget(Message) (Components|GetOwner)))
      (if _returnvalue_2 ; We check this so we can\nface the correct direction, which\nis the target, if it exists.
        (bind _facing_rotation (Class|BPILPSPCHAI|LPSP,AI-GetChaseTargetFacingRotation(Message) (Components|GetOwner)))
        (CallFunction|EventSmoothlySetRootYawMovingSmooth (Math|Rotator|SelectRotator (CallFunction|LPSP-SubtractRotators (Math|Rotator|MakeRotator 0.0 (.Pitch (Math|Rotator|BreakRotator _facing_rotation)) (.Yaw (Math|Rotator|BreakRotator _facing_rotation))) "0,90.000000, 0") (LocalVariables|GetAdjusted%20Velocity%20Rotation) (or (Variables|InfimaGames|Data|GetAiming) (Variables|InfimaGames|Data|GetUnarmed))))
        (else
          (CallFunction|EventSmoothlySetRootYawMovingSmooth (LocalVariables|GetAdjusted%20Velocity%20Rotation)))))
    (:then_1
      (return))))

(fn AIUpdateLook
  (bind _root_yaw_moving_smooth (Variables|InfimaGames|Data|GetRoot%20Yaw%20Moving%20Smooth))
  (bind (_roll _pitch _yaw) (Math|Rotator|BreakRotator _root_yaw_moving_smooth))
  (Utilities|FlowControl|Sequence
    (:then_0
      (bind _facing_rotation (Class|BPILPSPCHAI|LPSP,AI-GetChaseTargetFacingRotation(Message) (Components|GetOwner)))
      (CallFunction|EventAllSetLookMoving (Math|Rotator|MakeRotator (* (.Pitch (Math|Rotator|BreakRotator (Math|Rotator|Delta(Rotator) _facing_rotation (Math|Rotator|MakeRotator _roll _pitch _yaw)))) -1.0) 0.0 (- (.Yaw (Math|Rotator|BreakRotator (Math|Rotator|Delta(Rotator) _facing_rotation (Math|Rotator|MakeRotator _roll _pitch _yaw)))) 9e+01))))
    (:then_1
      (return))))