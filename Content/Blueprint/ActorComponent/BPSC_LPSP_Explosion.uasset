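; Explosion scene component that applies damage, physics impulses and indexed world camera shakes from its location.
; Radius is randomized on BeginPlay, while damage and impulse strength are rolled within ranges when applied.
; Damage and impulse each select Point mode, using a supplied hit result, or Radial mode around the component.
; Radial impulse pushes overlapped actors' primitives and Character capsules, optionally skipping actors blocked by a line-of-sight trace.
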(event EventBeginPlay
  (bind _radius (Variables|InfimaGames|LowPolyShooterPack|ExplosionComponent|GeneralSettings|GetRadius))
  ;[1 0 0 1 12] Begin Play
  (|CallParentFunction)
  (Variables|InfimaGames|LowPolyShooterPack|Data|SetRadius%20Value (Math|Random|RandomFloatinRange (.x _radius) (.y _radius))))

(fn ApplyPointImpulse
  (params (Result :type Hit%20Result%20Structure))
  (bind (_bblockinghit _binitialoverlap _time _distance _location _impactpoint _normal _impactnormal _physmat _hitactor _hitcomponent _hitbonename) (Collision|BreakHitResult Result))
  (bind (_bblockinghit_2 _binitialoverlap_2 _time_2 _distance_2 _location_2 _impactpoint_2 _normal_2 _impactnormal_2 _physmat_2 _hitactor_2 _hitcomponent_2 _hitbonename_2 _bonename _hititem _elementindex _faceindex _tracestart _traceend) (Collision|BreakHitResult Result))
  (Utilities|FlowControl|Sequence
    (:then_0
      (return))
    (:then_1
      (if (.bBlockingHit (Collision|BreakHitResult Result))
        (if (not (or (not (Variables|InfimaGames|LowPolyShooterPack|ExplosionComponent|Impulse|GetImpulse)) (Utilities|Enum|Equal(Enum) (Variables|InfimaGames|LowPolyShooterPack|ExplosionComponent|Impulse|GetImpulse%20Method) "NewEnumerator1")))
          (bind _output_get (LocalVariables|SetComponent (.HitComponent (Collision|BreakHitResult Result))))
          (Utilities|IsValid _output_get
            (:Is%20Valid
              (LocalVariables|SetHit%20Bone (.HitBoneName (Collision|BreakHitResult Result)))
              (if (Physics|IsSimulatingPhysics (LocalVariables|GetComponent) (LocalVariables|GetHit%20Bone))
                (bind _output_get_2 (LocalVariables|SetDirection (- _tracestart _traceend)))
                (LocalVariables|SetDirection (Math|Vector|Normalize _output_get_2))
                (Physics|AddImpulseatLocation (LocalVariables|GetComponent) (* (* (LocalVariables|GetDirection) (InfimaGames|LowPolyShooterPack|ExplosionComponent|GetImpulse)) -1.0) _location _hitbonename)))))))))

(fn ApplyRadialImpulse
  (params (Multiplier :type Float%20%28double-precision%29))
  (Utilities|FlowControl|Sequence
    (:then_0
      (LocalVariables|SetUsed%20Impulse (* (InfimaGames|LowPolyShooterPack|ExplosionComponent|GetImpulse) Multiplier))
      (Utilities|Array|Add (LocalVariables|GetIgnored%20Actors) (Components|GetOwner))
      (bind _outactors (Collision|SphereOverlapActors (Transformation|GetWorldLocation) (Variables|InfimaGames|LowPolyShooterPack|Data|GetRadius%20Value) (Variables|InfimaGames|LowPolyShooterPack|ExplosionComponent|Impulse|GetImpulse%20Object%20Types) 0 (LocalVariables|GetIgnored%20Actors)))
      (for _array_element _outactors
        (LocalVariables|SetCurrent _array_element)
        (if (or (not (Variables|InfimaGames|LowPolyShooterPack|ExplosionComponent|Impulse|GetUse%20Impulse%20Prevention)) (InfimaGames|LowPolyShooterPack|ExplosionComponent|CanHitActor (LocalVariables|GetCurrent) (Variables|InfimaGames|LowPolyShooterPack|ExplosionComponent|Impulse|GetImpulsePreventionChannel) (Variables|InfimaGames|LowPolyShooterPack|ExplosionComponent|Debug|GetbDebugRadialDamagePrevention) (* (Math|Vector|VectorUp) 1e+01)))
          (bind _ascharacter (Utilities|Casting|CastToCharacter (LocalVariables|GetCurrent))
            (:then
              (bind _output_get (LocalVariables|SetCharacter _ascharacter))
              (Utilities|IsValid _output_get
                (:Is%20Valid
                  (Utilities|IsValid (Variables|/Script/Engine.Actor|GetRootComponent (LocalVariables|GetCharacter))
                    (:Is%20Valid
                      (Physics|AddRadialImpulse (Variables|/Script/Engine.Character|GetCapsuleComponent (LocalVariables|GetCharacter)) (Transformation|GetWorldLocation) (Variables|InfimaGames|LowPolyShooterPack|Data|GetRadius%20Value) (LocalVariables|GetUsed%20Impulse) (Variables|InfimaGames|LowPolyShooterPack|ExplosionComponent|Impulse|GetImpulse%20Falloff) false))))
                (:Is%20Not%20Valid
                  _)))
            (:CastFailed
              _))
          (for _array_element_2 (Actor|GetComponentsByClass (LocalVariables|GetCurrent) "/Script/Engine.PrimitiveComponent")
            (bind _asprimitive_component (Utilities|Casting|CastToPrimitiveComponent _array_element_2))
            (Physics|AddRadialImpulse _asprimitive_component (Transformation|GetWorldLocation) (Variables|InfimaGames|LowPolyShooterPack|Data|GetRadius%20Value) (LocalVariables|GetUsed%20Impulse) (Variables|InfimaGames|LowPolyShooterPack|ExplosionComponent|Impulse|GetImpulse%20Falloff) false)))))
    (:then_1
      (return))))

(fn GetImpulse
  (bind _impulse_force (Variables|InfimaGames|LowPolyShooterPack|ExplosionComponent|Impulse|GetImpulse%20Force))
  (return (Math|Random|RandomFloatinRange (.x _impulse_force) (.y _impulse_force))))

(fn CanHitActor
  (params (Arg%20Actor :type Actor%20Object%20Reference) (Channel :type ETraceTypeQuery%20Enum :default "TraceTypeQuery1") (debug :type Boolean) (Offset :type Vector :default "0.000000,0,0"))
  (Utilities|FlowControl|Sequence
    (:then_0
      (Utilities|Array|Add (LocalVariables|GetIgnored) (Components|GetOwner))
      (Utilities|Array|Add (LocalVariables|GetIgnored) Arg%20Actor)
      (bind _returnvalue (Collision|LineTraceByChannel (+ (Transformation|GetWorldLocation) Offset) (+ (Transformation|GetActorLocation Arg%20Actor) Offset) Channel false (LocalVariables|GetIgnored) (select debug "ForDuration" "None")))
      (return (not _returnvalue)))
    (:then_1
      (return false))))

(fn ApplyPointDamage
  (params (Damage%20Causer :type Actor%20Object%20Reference) (Event%20Causer :type Controller%20Object%20Reference) (Result :type Hit%20Result%20Structure))
  (bind _hitactor (Collision|BreakHitResult Result))
  (Utilities|FlowControl|Sequence
    (:then_0
      (if (.bBlockingHit (Collision|BreakHitResult Result))
        (if (and (Variables|InfimaGames|LowPolyShooterPack|ExplosionComponent|Damage|GetDamage) (Utilities|Enum|Equal(Enum) (Variables|InfimaGames|LowPolyShooterPack|ExplosionComponent|Damage|GetDamage%20Method) "NewEnumerator0"))
          (Utilities|IsValid _hitactor
            (:Is%20Valid
              (if (Variables|/Script/Engine.Actor|GetbCanBeDamaged _hitactor)
                (Game|Damage|ApplyPointDamage (.HitActor (Collision|BreakHitResult Result)) (InfimaGames|LowPolyShooterPack|ExplosionComponent|GetDamage) (Math|Vector|MakeVector 0.0 0.0 0.0) Result Event%20Causer Damage%20Causer)))))))
    (:then_1
      (return))))

(fn ApplyRadialDamage
  (params (Damage%20Causer :type Actor%20Object%20Reference))
  (Utilities|FlowControl|Sequence
    (:then_0
      (if (not (or (not (Variables|InfimaGames|LowPolyShooterPack|ExplosionComponent|Damage|GetDamage)) (Utilities|Enum|Equal(Enum) (Variables|InfimaGames|LowPolyShooterPack|ExplosionComponent|Damage|GetDamage%20Method) "NewEnumerator0")))
        (Utilities|Array|Add (LocalVariables|GetIgnored%20Actors) (Components|GetOwner))
        (Game|Damage|ApplyRadialDamage (InfimaGames|LowPolyShooterPack|ExplosionComponent|GetDamage) (Transformation|GetWorldLocation) (Variables|InfimaGames|LowPolyShooterPack|Data|GetRadius%20Value) "/Script/Engine.DamageType" (LocalVariables|GetIgnored%20Actors) Damage%20Causer 0 false "ECC_Visibility")))
    (:then_1
      (return))))

(fn StartShake
  (params (index :type Integer))
  (Utilities|FlowControl|Sequence
    (:then_0
      (if (Variables|InfimaGames|LowPolyShooterPack|ExplosionComponent|Shake|GetShake)
        (if (and (Utilities|Array|IsValidIndex (Variables|InfimaGames|LowPolyShooterPack|ExplosionComponent|Shake|GetShakes) index) (Utilities|IsValidClass (Utilities|Array|Get(acopy) (Variables|InfimaGames|LowPolyShooterPack|ExplosionComponent|Shake|GetShakes) index)))
          (Camera|PlayWorldCameraShake (Utilities|Array|Get(acopy) (Variables|InfimaGames|LowPolyShooterPack|ExplosionComponent|Shake|GetShakes) index) (Transformation|GetWorldLocation) (Variables|InfimaGames|LowPolyShooterPack|ExplosionComponent|Shake|GetShake%20Inner%20Radius) (Variables|InfimaGames|LowPolyShooterPack|ExplosionComponent|Shake|GetShake%20Outer%20Radius) (Variables|InfimaGames|LowPolyShooterPack|ExplosionComponent|Shake|GetShake%20Falloff)))))
    (:then_1
      (return))))

(fn DrawDebugRadius
  (params (Color :type Linear%20Color%20Structure) (Duration :type Float%20%28double-precision%29))
  (if (== (Variables|InfimaGames|LowPolyShooterPack|Data|GetRadius%20Value) 0.0)
    (return)
    (else
      (Rendering|Debug|DrawDebugSphere (Transformation|GetWorldLocation) (Variables|InfimaGames|LowPolyShooterPack|Data|GetRadius%20Value) 12 Color Duration))))

(fn TryApplyImpulse
  (params (Multiplier :type Float%20%28double-precision%29) (Result :type Hit%20Result%20Structure))
  (Utilities|FlowControl|Sequence
    (:then_0
      (if (not (not (Variables|InfimaGames|LowPolyShooterPack|ExplosionComponent|Impulse|GetImpulse)))
        (switch Utilities|FlowControl|Switch|SwitchonE_LPSP_Damage_Type (Variables|InfimaGames|LowPolyShooterPack|ExplosionComponent|Impulse|GetImpulse%20Method)
          (:NewEnumerator0
            (InfimaGames|LowPolyShooterPack|ExplosionComponent|ApplyPointImpulse Result))
          (:NewEnumerator1
            (InfimaGames|LowPolyShooterPack|ExplosionComponent|ApplyRadialImpulse Multiplier)))))
    (:then_1
      (return))))

(fn TryApplyDamage
  (params (Result :type Hit%20Result%20Structure))
  (Utilities|FlowControl|Sequence
    (:then_0
      (switch Utilities|FlowControl|Switch|SwitchonE_LPSP_Damage_Type (Variables|InfimaGames|LowPolyShooterPack|ExplosionComponent|Damage|GetDamage%20Method)
        (:NewEnumerator0
          (InfimaGames|LowPolyShooterPack|ExplosionComponent|ApplyPointDamage (Components|GetOwner) 0 Result))
        (:NewEnumerator1
          (InfimaGames|LowPolyShooterPack|ExplosionComponent|ApplyRadialDamage))))
    (:then_1
      (return))))

(fn GetRadiusValue
  (return (Variables|InfimaGames|LowPolyShooterPack|Data|GetRadius%20Value)))

(fn GetDamage
  (bind _damage_amount (Variables|InfimaGames|LowPolyShooterPack|ExplosionComponent|Damage|GetDamage%20Amount))
  (return (Math|Random|RandomFloatinRange (.x _damage_amount) (.y _damage_amount))))