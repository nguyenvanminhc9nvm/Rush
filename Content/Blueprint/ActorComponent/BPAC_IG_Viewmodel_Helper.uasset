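; Actor component that switches its owner's meshes between world and first-person viewmodel rendering.
; Setting or refreshing the viewmodel mode updates every mesh component on the owner.
; Each mesh gets a "Field Of View Alpha" material scalar of 0 or 1, driving a material-based FOV effect, plus a bounds scale matching the mode.
; The Viewmodel RepNotify handler is empty, so only those two events apply changes.
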(event Custom|Event%20Set%20Viewmodel
  (params (Viewmodel :type E_LPSP_Viewmodel%20Enum :default "NewEnumerator1"))
  ;[1 0 0.5349 1 12] Set Viewmodel
  (Variables|InfimaGames|Data|SetViewmodel Viewmodel)
  (InfimaGames|ViewmodelHelper|UpdateMeshes))

(event Custom|Event%20Refresh%20Viewmodel
  ;[1 0 0.1355 1 12] Refresh Viewmodel
  (InfimaGames|ViewmodelHelper|UpdateMeshes))

(fn UpdateMeshes
  (Utilities|FlowControl|Sequence
    (:then_0
      (for _array_element (Actor|GetComponentsByClass (Components|GetOwner) "/Script/Engine.MeshComponent")
        (bind _output_get (LocalVariables|SetLocal%20Mesh _array_element))
        (Utilities|IsValid _output_get
          (:Is%20Valid
            (Rendering|Material|SetScalarParameterValueonMaterials (LocalVariables|GetLocal%20Mesh) "Field Of View Alpha" (Utilities|Select :Index (Variables|InfimaGames|Data|GetViewmodel) :NewEnumerator1 0.0 :NewEnumerator0 1.0))
            (Rendering|SetBoundsScale (LocalVariables|GetLocal%20Mesh) (Utilities|Select :Index (Variables|InfimaGames|Data|GetViewmodel) :NewEnumerator1 (Variables|Config|GetWorld%20Bounds%20Scale) :NewEnumerator0 (Variables|Config|GetViewmodel%20Bounds%20Scale)))))))
    (:then_1
      (return))))

(fn OnRepViewmodel)