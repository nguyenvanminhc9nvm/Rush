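; Actor component that tracks a character's stamina for running and jumping, starting at the maximum.
; On the local owner's tick, stamina drains while running and regenerates otherwise; hitting zero pauses these updates for a few seconds via a timer.
; Changes apply locally, then replicate through a server event that multicasts the value.
; Functions expose the stamina percentage, deduct jump cost and check whether a jump is affordable.
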(event Custom|Event%20Server%20Set%20Stamina
  (params (Value :type Float%20%28double-precision%29))
  ;[0.3517 1 0.6823 1 12] Set Stamina
  (CallFunction|EventMulticastSetStamina Value))

(event Custom|Event%20Set%20Stamina
  (params (Value :type Float%20%28double-precision%29))
  ;[0.3517 1 0.6823 1 12] Set Stamina
  (bind _output_get (Variables|Data|SetStamina Value))
  (CallFunction|EventServerSetStamina _output_get))

(event Custom|Event%20Unblock%20Stamina%20Updates
  ;[0.8749 1 0.1894 1 12] Unblock Stamina Updates
  (Variables|Data|SetBlocked%20Stamina%20Updates false))

(event Custom|Event%20Multicast%20Set%20Stamina
  (params (Value :type Float%20%28double-precision%29))
  ;[0.3517 1 0.6823 1 12] Set Stamina
  (Variables|Data|SetStamina Value))

(event EventTick
  (params (DeltaSeconds :type Float%20%28single-precision%29))
  (|CallParentFunction DeltaSeconds)
  (bind _local (Class|BPILPSPPCH|LPSP-IsLocal(Message) (Components|GetOwner)))
  (if _local
    (if (not (Variables|Data|GetBlocked%20Stamina%20Updates))
      (bind _returnvalue (Class|BPILPSPPCH|LPSP-IsRunning(Message) (Components|GetOwner)))
      (Variables|Data|SetRunning _returnvalue)
      (CallFunction|EventSetStamina (Math|Float|Clamp(Float) (+ (Variables|Data|GetStamina) (* (Utilities|Time|GetWorldDeltaSeconds) (Math|Float|SelectFloat -1.0 1.0 (Variables|Data|GetRunning)))) 0.0 (Variables|Config|GetMax%20Stamina)))
      (Utilities|FlowControl|Sequence
        (:then_0
          (if (and (== (Variables|Data|GetStamina) 0.0) (!= (Variables|Data|GetStamina) (Variables|Data|GetLast%20Frame%20Stamina)))
            (Variables|Data|SetBlocked%20Stamina%20Updates true)
            (Utilities|Time|SetTimerbyEvent (EventDispatchers|CreateEvent :!event Custom|Event%20Unblock%20Stamina%20Updates) 3.0)))
        (:then_1
          (Variables|Data|SetLast%20Frame%20Stamina (Variables|Data|GetStamina)))))))

(event EventBeginPlay
  ;[1 0.2783 0.1462 1 12] Begin Play
  (|CallParentFunction)
  (Variables|Data|SetStamina (Variables|Config|GetMax%20Stamina)))

(fn GetStaminaPercent
  (return (/ (Variables|Data|GetStamina) (Variables|Config|GetMax%20Stamina))))

(fn Jump
  (CallFunction|EventSetStamina (- (Variables|Data|GetStamina) (Variables|Config|GetJump%20Stamina%20Cost)))
  (return))

(fn CanJump
  (return (> (- (Variables|Data|GetStamina) (Variables|Config|GetJump%20Stamina%20Cost)) 0.0)))