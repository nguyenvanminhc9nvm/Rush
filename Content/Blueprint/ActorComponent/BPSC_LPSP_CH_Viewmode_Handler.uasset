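; Pawn component that switches its owner between first and third person viewmodes, applying a starting mode on possession.
; Changes are set locally and sent to the server, with the Viewmode RepNotify broadcasting the change and running setup.
; Setup reattaches inventory and left-hand socket to viewmodel arms or full-body mesh (always full-body for AI and remote pawns), adjusts spring-arm lag and messages the pawn to refresh item physics and FOV materials.
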(event Custom|Event%20Owner%20Posessed
  ;[0.1405 1 0 1 12] Event Owner Posessed
  (CallFunction|EventAllUpdateViewmode (Variables|Config|GetStarting%20Viewmode)))

(event Custom|Event%20Update%20Viewmode
  (params (New%20Viewmode :type E_LPSP_Viewmode%20Enum :default "NewEnumerator0"))
  ;[0.7113 1 0 1 12] Event Update Viewmode
  (Variables|Data|SetPrev%20Viewmode (Variables|Data|GetViewmode))
  (Variables|Data|SetViewmode New%20Viewmode))

(event Custom|Event%20%28All%29%20Toggle%20Viewmode
  ;[0.8601 1 0 1 12] Event (All) Toggle Viewmode
  (CallFunction|EventAllUpdateViewmode (Utilities|Select :Index (CallFunction|GetViewmodePure) :NewEnumerator2 "NewEnumerator0" :NewEnumerator0 "NewEnumerator1" :NewEnumerator1 "NewEnumerator0")))

(event Custom|Event%20Update%20Viewmode%20Setup
  ;[0.2297 1 0 1 12] Event Update Viewmode Setup
  (Default|CallOnUpdateViewmode (Variables|Data|GetPrev%20Viewmode) (Variables|Data|GetViewmode))
  (Transformation|AttachComponentToComponent (CallFunction|GetInventoryPure) (CallFunction|GetInventoryAttachComponentPure) "SOCKET_Weapon" "SnapToTarget" "SnapToTarget" "SnapToTarget" false)
  (|CGraphAttachLeftHandSocket)
  (CallFunction|UpdateOwnerSpringArmSettings)
  (Class|BPILPSPPCH|LPSP-UpdateEquippedItemPhysicalSettings(Message) (CallFunction|GetOwningPawnPure))
  (Class|BPILPSPPCH|LPSP-UpdateFieldOfViewMaterials(Message) (CallFunction|GetOwningPawnPure)))

(event Custom|Event%20All%20Update_Viewmode
  (params (New%20Viewmode :type E_LPSP_Viewmode%20Enum :default "NewEnumerator0"))
  ;[0.8406 1 0 1 12] All Update Viewmode
  (CallFunction|EventUpdateViewmode New%20Viewmode)
  (CallFunction|Event(Server)UpdateViewmode New%20Viewmode))

(event Custom|Event%20%28Server%29%20Update%20Viewmode
  (params (New%20Viewmode :type E_LPSP_Viewmode%20Enum :default "NewEnumerator0"))
  ;[0.05499 1 0 1 12] Event (Server) Update Viewmode
  (CallFunction|EventUpdateViewmode New%20Viewmode))

(fn GetInventoryAttachComponentPure
  (bind _returnvalue (CallFunction|GetAnimatedViewmodelArms))
  (return (select (and (Pawn|IsLocallyControlled (CallFunction|GetOwningPawnPure)) (not (CallFunction|IsOwnerAI))) (Utilities|Select :Index (Variables|Data|GetViewmode) :NewEnumerator2 _returnvalue :NewEnumerator0 _returnvalue :NewEnumerator1 (CallFunction|GetAnimatedFull-BodyCharacter)) (CallFunction|GetAnimatedFull-BodyCharacter))))

(fn GetViewmodePure
  (return (Variables|Data|GetViewmode)))

(fn GetPreviousViewmodePure
  (return (Variables|Data|GetPrev%20Viewmode)))

(fn GetOwningPawnPure
  (Utilities|FlowControl|Sequence
    (:then_0
      (Utilities|IsValid (Variables|Data|GetOwning%20Pawn)
        (:Is%20Valid
          (return (Variables|Data|GetOwning%20Pawn)))))
    (:then_1
      (bind _aspawn (Utilities|Casting|CastToPawn (Components|GetOwner)))
      (bind _output_get (Variables|Data|SetOwning%20Pawn _aspawn))
      (return _output_get))))

(fn GetInventoryPure
  (Utilities|FlowControl|Sequence
    (:then_0
      (Utilities|IsValid (Variables|Default|GetInventory)
        (:Is%20Valid
          (return (Variables|Default|GetInventory)))))
    (:then_1
      (bind _output_get (Variables|Default|SetInventory (Utilities|Array|Get(acopy) (Actor|GetComponentsbyTag (CallFunction|GetOwningPawnPure) "/Script/Engine.SceneComponent" "Inventory_Component_Parent"))))
      (return _output_get))))

(fn OnRepViewmode
  (CallFunction|EventUpdateViewmodeSetup))

(fn GetAnimatedViewmodelArms
  (bind _returnvalue (Components|GetOwner))
  (bind _returnvalue_2 (Actor|GetComponentsbyTag _returnvalue "/Script/Engine.SkeletalMeshComponent" "Animated Viewmodel Arms"))
  (Utilities|IsValid (Variables|Default|GetAnimated%20Viewmodel%20Arms)
    (:Is%20Valid
      (return (Variables|Default|GetAnimated%20Viewmodel%20Arms)))
    (:Is%20Not%20Valid
      (LocalVariables|SetComponents _returnvalue_2)
      (if (Utilities|Array|IsValidIndex _returnvalue_2)
        (bind _output_get (Variables|Default|SetAnimated%20Viewmodel%20Arms (Utilities|Array|Get(acopy) _returnvalue_2)))
        (return _output_get)))))

(fn GetAnimatedFull-BodyCharacter
  (Utilities|IsValid (Variables|Default|GetAnimated%20Full-Body%20Character)
    (:Is%20Valid
      (return (Variables|Default|GetAnimated%20Full-Body%20Character)))
    (:Is%20Not%20Valid
      (bind _output_get (Variables|Default|SetAnimated%20Full-Body%20Character (Utilities|Array|Get(acopy) (Actor|GetComponentsbyTag (Components|GetOwner) "/Script/Engine.SkeletalMeshComponent" "Animated Full-Body Character"))))
      (return _output_get))))

(fn UpdateOwnerSpringArmSettings
  (Utilities|FlowControl|Sequence
    (:then_0
      (bind _output_get (LocalVariables|SetOwner%20Spring%20Arm (Utilities|Array|Get(acopy) (Actor|GetComponentsbyTag (Components|GetOwner) "/Script/Engine.SpringArmComponent" "Main Spring Arm"))))
      (Utilities|IsValid _output_get
        (:Is%20Valid
          (bind _output_get_2 (Variables|/Script/Engine.SpringArmComponent|SetbEnableCameraRotationLag (LocalVariables|GetOwner%20Spring%20Arm) (Utilities|Select :Index (CallFunction|GetViewmodePure) :NewEnumerator2 false :NewEnumerator0 false :NewEnumerator1 true)))
          (bind _output_get_3 (Variables|/Script/Engine.SpringArmComponent|SetbEnableCameraLag (LocalVariables|GetOwner%20Spring%20Arm) _output_get_2))
          (Variables|/Script/Engine.SceneComponent|SetbAbsoluteRotation (LocalVariables|GetOwner%20Spring%20Arm) _output_get_3))))
    (:then_1
      (return))))

(fn IsOwnerAI
  (bind _returnvalue (Class|BPILPSPPCH|LPSP-IsAI(Message) (CallFunction|GetOwningPawnPure)))
  (return _returnvalue))